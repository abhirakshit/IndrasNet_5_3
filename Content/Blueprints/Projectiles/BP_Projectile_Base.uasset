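; Base projectile Blueprint that moves via a ProjectileMovement component and reports impacts through an OnProjectileHit dispatcher.
; The construction script runs StartProjectile, which applies Speed, Gravity and local-space Direction to the movement component and prints those values for debugging.
; Sphere collision hits broadcast the other actor and hit result.
; A physics-impulse-and-destroy branch is left disconnected, and the actor Hit event is empty.
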(event `self.SphereCollision.OnComponentHit`
  (params (HitComponent :type "PrimitiveComponent Object Reference") (OtherActor :type "Actor Object Reference") (OtherComp :type "PrimitiveComponent Object Reference") (NormalImpulse :type "Vector Structure") (Hit :type "HitResult Structure (by ref)"))
  (`self.OnProjectileHit` OtherActor Hit))

(event `self.ReceiveHit`
  (params (MyComp :type "PrimitiveComponent Object Reference") (Other :type "Actor Object Reference") (OtherComp :type "PrimitiveComponent Object Reference") (bSelfMoved :type Boolean) (HitLocation :type "Vector Structure") (HitNormal :type "Vector Structure") (NormalImpulse :type "Vector Structure") (Hit :type "HitResult Structure (by ref)")))

(fn `StartProjectile`
  (bind _projectilemovement (`self.ProjectileMovement`))
  (bind _speed (`self.Speed`))
  (`|ExecutionSequence`
    (:`then_0`
      (set `ProjectileMovementComponent.InitialSpeed` _speed _projectilemovement))
    (:`then_1`
      (set `ProjectileMovementComponent.MaxSpeed` _speed _projectilemovement))
    (:`then_2`
      (set `ProjectileMovementComponent.ProjectileGravityScale` (`self.Gravity`) _projectilemovement))
    (:`then_3`
      (`ProjectileMovementComponent.SetVelocityInLocalSpace` _projectilemovement (`self.Direction`)))
    (:`then_4`
      (`KismetSystemLibrary.PrintText` (`|FormatText` "BP Projectile base: {speed}, {gravity}, {direction}" (`self.Speed`) (`self.Gravity`) (`KismetStringLibrary.Conv_VectorToString` (`self.Direction`))) true true (struct :`G` 0.66 :`B` 1.0 :`A` 1.0) 5.0))))

(fn `UserConstructionScript`
  (`self.StartProjectile`))