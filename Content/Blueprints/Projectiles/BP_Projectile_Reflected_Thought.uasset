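; BP_Projectile_Reflected_Thought is a projectile that sets off an explosion when it hits a destructible component.
; On Hit, it checks for the misspelled "Desctructible" component tag, spawns a BP_Bomb at the impact point, explodes it immediately and prints a debug message.
; The sphere collision's "repressionBP" tag check leads to nothing, and DestroyActor is disconnected.
; GetProjectileVelocity exposes the movement component's velocity.
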(event `self.ReceiveHit`
  (params (MyComp :type "PrimitiveComponent Object Reference") (Other :type "Actor Object Reference") (OtherComp :type "PrimitiveComponent Object Reference") (bSelfMoved :type Boolean) (HitLocation :type "Vector Structure") (HitNormal :type "Vector Structure") (NormalImpulse :type "Vector Structure") (Hit :type "HitResult Structure (by ref)"))
  (if (`ActorComponent.ComponentHasTag` OtherComp "Desctructible")
    (bind _returnvalue (`|SpawnActorFromClass` "/Game/Blueprints/Repression/BP_Bomb.BP_Bomb_C" (`KismetMathLibrary.MakeTransform` HitLocation) "Undefined" "MultiplyWithRoot" null 0.2 50000.0 2.0 null))
    (`/Game/Blueprints/Repression/BP_Bomb.Explode` _returnvalue)
    (`KismetSystemLibrary.PrintText` "Boom")))

(event `self.SphereCollision.OnComponentHit`
  (params (HitComponent :type "PrimitiveComponent Object Reference") (OtherActor :type "Actor Object Reference") (OtherComp :type "PrimitiveComponent Object Reference") (NormalImpulse :type "Vector Structure") (Hit :type "HitResult Structure (by ref)"))
  (if (`self.ActorHasTag` OtherActor "repressionBP")
    _))

(fn `GetProjectileVelocity`
  (returns (Velocity :type "Vector Structure"))
  (return (`MovementComponent.Velocity` (`self.ProjectileMovement`))))

(fn `UserConstructionScript`
  (`parent.UserConstructionScript`))