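; Mental-model visual actor with an inner light, an outer mask shell and three toggleable, tinted repression meshes.
; Events step the inner light's emissive "withdrawal" value and play or reverse a timeline that dissolves the shell via dynamic materials, with optional randomised light intensity and colour at BeginPlay.
; SpawnConnections links it to nearby supplied locations with random-coloured Niagara arc beams, capped by count and random distance, deactivated on destruction.
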(event `self.ReceiveDestroyed`
  (for _array_element (`self.ConnectionsArray`)
    (`ActorComponent.Deactivate` _array_element)
    (`NiagaraComponent.SetAutoDestroy` _array_element true)))

(event `self.ReceiveBeginPlay`
  (`|ExecutionSequence`
    (:`then_0`
      (`self.toggleRepressions`))
    (:`then_1`
      (`self.updateWithdrawal` (`self.withdrawalVal`)))
    (:`then_2`
      (if (`self.setRandomProps`)
        (`self.setRandomPropValues`)))))

(event `/Game/Blueprints/Interfaces/BP_MentalModelInterface.addNewOuterShell`
  (bind _maskshell (`self.MaskShell`))
  (bind _returnvalue (`PrimitiveComponent.CreateDynamicMaterialInstance` _maskshell 0 (`PrimitiveComponent.GetMaterial` _maskshell 0) "None"))
  (`KismetSystemLibrary.PrintText` "Add Shield")
  (bind (_direction _shieldon) (`Timeline|ShieldAnimate` :!label _label)
    (:`Update`
      (`MaterialInstanceDynamic.SetScalarParameterValue` _returnvalue "DissolveAmount" _shieldon))))

(event `/Game/Blueprints/Interfaces/BP_MentalModelInterface.removeOutermostShell`
  (bind _maskshell (`self.MaskShell`))
  (`PrimitiveComponent.CreateDynamicMaterialInstance` _maskshell 0 (`PrimitiveComponent.GetMaterial` _maskshell 0) "None")
  (`KismetSystemLibrary.PrintText` "Remove Shield")
  (goto _label :!via `Reverse`))

(event `/Game/Blueprints/Interfaces/BP_MentalModelInterface.toggleShowHideRepressions`
  (set `self.showingRepression?` (not (`self.showingRepression?`)))
  (`self.toggleRepressions`))

(event `/Game/Blueprints/Interfaces/BP_MentalModelInterface.increaseInnerLight`
  (if (`self.showInnerLight?`)
    (bind _output_get (set `self.withdrawalVal` (+ (`self.withdrawalVal`) (`self.incrementVal`))))
    (`self.updateWithdrawal` _output_get)))

(event `/Game/Blueprints/Interfaces/BP_MentalModelInterface.decreaseInnerLIght`
  (if (`self.showInnerLight?`)
    (bind _output_get (set `self.withdrawalVal` (- (`self.withdrawalVal`) (`self.incrementVal`))))
    (`self.updateWithdrawal` _output_get)))

(fn `getModelProperties`
  (returns (props :type "/Game/Blueprints/Structs/ST_MentalModelProperties Structure"))
  (return))

(fn `setRandomPropValues`
  (bind _il_mesh (`self.IL_Mesh`))
  (`|ExecutionSequence`
    (:`then_0`
      (`self.updateWithdrawal` (`KismetMathLibrary.RandomFloatInRange` 100.0 1000.0)))
    (:`then_1`
      (bind _returnvalue (`PrimitiveComponent.CreateDynamicMaterialInstance` _il_mesh 0 (`PrimitiveComponent.GetMaterial` _il_mesh 0) "None"))
      (`MaterialInstanceDynamic.SetVectorParameterValue` _returnvalue "Color" (`KismetMathLibrary.MakeColor` (`KismetMathLibrary.RandomFloatInRange` 0.0 1.0) (`KismetMathLibrary.RandomFloatInRange` 0.0 1.0) (`KismetMathLibrary.RandomFloatInRange` 0.0 1.0))))))

(fn `SpawnConnections`
  (params (MMLocationsArray :type "Array of Vector Structure"))
  (locals (J :type "Vector Structure") (Distance :type "Float (double-precision)") (MinConnectionDistance :type "Float (double-precision)" :default 200.0) (CurrentPoint :type "Vector Structure") (MaxConnections :type Integer :default 1) (MinConnectionDistance1 :type "Float (double-precision)" :default 300.0))
  (set `local.CurrentPoint` (`SceneComponent.K2_GetComponentLocation` (`self.DefaultSceneRoot`)))
  (for _array_element MMLocationsArray
    (if (<= (`KismetArrayLibrary.Array_Length` (`self.ConnectionsArray`)) (`local.MaxConnections`))
      (bind _output_get (set `local.J` _array_element))
      (set `local.Distance` (`KismetMathLibrary.Vector_Distance` _output_get (`local.CurrentPoint`)))
      (if (and (> (`local.Distance`) 0.0) (<= (`local.Distance`) (`KismetMathLibrary.RandomFloatInRange` (`local.MinConnectionDistance`) (`local.MinConnectionDistance1`))))
        (bind _returnvalue (`NiagaraFunctionLibrary.SpawnSystemAtLocation` "/Game/Assets/ElectricArcs/NiagaraSystems/ElectricArcForBP/N_BP-FlatArc_Smooth1.N_BP-FlatArc_Smooth1" (`local.CurrentPoint`)))
        (`|ExecutionSequence`
          (:`then_0`
            (`NiagaraComponent.SetVariableVec3` _returnvalue "BeamEnd" (`local.J`)))
          (:`then_1`
            (`NiagaraComponent.SetVariableFloat` _returnvalue "Beam WidthMax" 1.0))
          (:`then_2`
            (`NiagaraComponent.SetVariableFloat` _returnvalue "Roundness" 2.0))
          (:`then_3`
            (`NiagaraComponent.SetVariableFloat` _returnvalue "LoopDurationMin" 1.0))
          (:`then_4`
            (`NiagaraComponent.SetVariableFloat` _returnvalue "LoopDurationMax" 1.5))
          (:`then_5`
            (`NiagaraComponent.SetVariableLinearColor` _returnvalue "Color" (`KismetMathLibrary.MakeColor` (`KismetMathLibrary.RandomFloat`) (`KismetMathLibrary.RandomFloat`) (`KismetMathLibrary.RandomFloat`))))
          (:`then_6`
            (`KismetArrayLibrary.Array_Add` (`self.ConnectionsArray`) _returnvalue)))))))

(fn `toggleRepressions`
  (bind _rep2 (`self.Rep2`))
  (bind _rep1 (`self.Rep1`))
  (bind _showingrepression_ (`self.showingRepression?`))
  (bind _rep3 (`self.Rep3`))
  (bind _returnvalue (`KismetMathLibrary.Conv_LinearColorToVector` (`self.repressionColor`)))
  (`|ExecutionSequence`
    (:`then_0`
      (`SceneComponent.SetVisibility` _rep3 _showingrepression_ false)
      (`SceneComponent.SetVisibility` _rep2 _showingrepression_ false)
      (`SceneComponent.SetVisibility` _rep1 _showingrepression_ false))
    (:`then_1`
      (`MeshComponent.SetVectorParameterValueOnMaterials` _rep3 "Inner_Color" _returnvalue)
      (`MeshComponent.SetVectorParameterValueOnMaterials` _rep3 "Outline_Color" _returnvalue)
      (`MeshComponent.SetVectorParameterValueOnMaterials` _rep2 "Inner_Color" _returnvalue)
      (`MeshComponent.SetVectorParameterValueOnMaterials` _rep2 "Outline_Color" _returnvalue)
      (`MeshComponent.SetVectorParameterValueOnMaterials` _rep1 "Inner_Color" _returnvalue)
      (`MeshComponent.SetVectorParameterValueOnMaterials` _rep1 "Outline_Color" _returnvalue))))

(fn `updateWithdrawal`
  (params (withdrawalVal :type "Float (double-precision)"))
  (locals (updateBrightnessValue :type "Float (double-precision)") (mi :type "MaterialInterface Object Reference"))
  (bind _il_mesh (`self.IL_Mesh`))
  (bind _returnvalue (`PrimitiveComponent.CreateDynamicMaterialInstance` _il_mesh 0 (`PrimitiveComponent.GetMaterial` _il_mesh 0) "None"))
  (`MaterialInstanceDynamic.SetScalarParameterValue` _returnvalue "emissiveColorMultiplier" withdrawalVal))

(fn `UserConstructionScript`)