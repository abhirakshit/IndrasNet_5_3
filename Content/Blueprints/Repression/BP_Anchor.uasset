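; BP_Anchor is a field system anchor that sets Chaos physics objects inside its collision box to static.
; Initialize adds a dynamic-state field command, culled to the box transform, on construction and BeginPlay.
; DecrementCollisionArea shrinks the box scale while MaxDecrement remains, prints debug text, reapplies the field and returns whether it shrank.
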(event `self.ReceiveBeginPlay`
  (`self.Initialize`))

(fn `Decrement Collision Area`
  (params (decrementVal :type "Float (double-precision)"))
  (returns (success :type Boolean))
  (bind (_returnvalue_location _returnvalue_rotation _returnvalue_scale) (`KismetMathLibrary.BreakTransform` (`SceneComponent.K2_GetComponentToWorld` (`self.BoxCollision`))))
  (bind _returnvalue (- _returnvalue_scale decrementVal))
  (if (> (`self.maxDecrement`) 0)
    (bind _result (`/Engine/EditorBlueprintResources/StandardMacros.DecrementInt` (`self.maxDecrement`))
      (:`  `
        (`KismetSystemLibrary.PrintText` (`|FormatText` "Dec: {d}, {s1}, {s2}" _result (`KismetStringLibrary.Conv_VectorToString` _returnvalue_scale) (`KismetTextLibrary.Conv_VectorToText` _returnvalue)))
        (`SceneComponent.K2_SetWorldTransform` (`self.BoxCollision`) (`KismetMathLibrary.MakeTransform` _returnvalue_location _returnvalue_rotation _returnvalue) false false)
        (`self.Initialize`)
        (return true)))
    (else
      (return false))))

(fn `Initialize`
  (`FieldSystemComponent.AddFieldCommand` (`self.FieldSystemComponent`) true "Field_DynamicState" null (`CullingField.SetCullingField` (`self.CullingField`) (`BoxFalloff.SetBoxFalloff` (`self.BoxFalloff`) 1.0 0.0 1.0 0.0 (`SceneComponent.K2_GetComponentToWorld` (`self.BoxCollision`)) "Field_FallOff_None") (`UniformInteger.SetUniformInteger` (`self.UniformInteger`) 3) "Field_Culling_Outside")))

(fn `UserConstructionScript`
  (`self.Initialize`))