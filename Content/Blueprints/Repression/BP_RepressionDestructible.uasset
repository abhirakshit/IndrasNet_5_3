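; Chaos destructible for the Repression feature that breaks loose when hit by an actor tagged "Dissolving Thought".
; On BeginPlay it registers a child BP_Anchor as an initialization field and randomizes rotation and scale.
; A qualifying hit decrements the anchor's collision area, removes all anchors and applies a kinematic field to free pieces at runtime.
; Removed pieces spawn sparkle Niagara effects, which are deactivated when the actor is destroyed.
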(event `self.ReceiveBeginPlay`
  (`|ExecutionSequence`
    (:`then_0`
      (`self.SetupAnchor`))
    (:`then_2`
      (`self.SetupTransform`))))

(event `self.GeometryCollection.OnComponentHit`
  (params (HitComponent :type "PrimitiveComponent Object Reference") (OtherActor :type "Actor Object Reference") (OtherComp :type "PrimitiveComponent Object Reference") (NormalImpulse :type "Vector Structure") (Hit :type "HitResult Structure (by ref)"))
  (bind _geometrycollection (`self.GeometryCollection`))
  (switch `name` (`|GetArrayItem` (`Actor.Tags` OtherActor))
    (:`dissolvingThought`
      (`KismetSystemLibrary.PrintText` "Hit")
      (bind _asbp_anchor (cast `/Game/Blueprints/Repression/BP_Anchor` (`ChildActorComponent.ChildActor` (`self.Anchor`))))
      (bind _success (`/Game/Blueprints/Repression/BP_Anchor.Decrement Collision Area` _asbp_anchor 1.0))
      (if _success
        _
        (else
          _))
      ;[1 1 1] Remove Anchor - https://forums.unrealengine.com/t/disabling-chaos-anchor-fields-at-runtime/496278
      (`GeometryCollectionComponent.RemoveAllAnchors` _geometrycollection)
      (`GeometryCollectionComponent.ApplyKinematicField` _geometrycollection 100.0 (`SceneComponent.K2_GetComponentLocation` _geometrycollection)))))

(event `self.GeometryCollection.OnChaosRemovalEvent`
  (params (RemovalEvent :type "ChaosRemovalEvent Structure (by ref)"))
  (`KismetSystemLibrary.PrintText` "Removal!")
  (bind _returnvalue (`NiagaraFunctionLibrary.SpawnSystemAtLocation` "/Game/Assets/FX-Niagara/NS_SparklingParticles.NS_SparklingParticles" RemovalEvent_Location))
  (`KismetArrayLibrary.Array_Add` (`self.NiagaraSystemObjs`) _returnvalue))

(event `self.GeometryCollection.OnComponentBeginOverlap`
  (params (OverlappedComponent :type "PrimitiveComponent Object Reference") (OtherActor :type "Actor Object Reference") (OtherComp :type "PrimitiveComponent Object Reference") (OtherBodyIndex :type Integer) (bFromSweep :type Boolean) (SweepResult :type "HitResult Structure (by ref)")))

(event `self.GeometryCollection.OnChaosBreakEvent`
  (params (BreakEvent :type "ChaosBreakEvent Structure (by ref)")))

(event `self.ReceiveDestroyed`
  (for _array_element (`self.NiagaraSystemObjs`)
    (`ActorComponent.Deactivate` _array_element)))

(fn `SetupAnchor`
  (bind _geometrycollection (`self.GeometryCollection`))
  (bind _asbp_anchor (cast `/Game/Blueprints/Repression/BP_Anchor` (`ChildActorComponent.ChildActor` (`self.Anchor`)))
    (:`then`
      (`KismetArrayLibrary.Array_Add` (`GeometryCollectionComponent.InitializationFields` (`self.GeometryCollection`)) _asbp_anchor)
      (`PrimitiveComponent.SetSimulatePhysics` _geometrycollection false)
      (`GeometryCollectionComponent.SetNotifyBreaks` _geometrycollection true)
      (`GeometryCollectionComponent.SetNotifyRemovals` _geometrycollection true)
      (`PrimitiveComponent.SetSimulatePhysics` _geometrycollection true))
    (:`CastFailed`
      (`KismetSystemLibrary.PrintText` "Anchor Cast Failed!"))))

(fn `SetupTransform`
  (bind _returnvalue (`KismetMathLibrary.RandomFloatInRange` 2.0 3.0))
  (`|ExecutionSequence`
    (:`then_0`
      (`SceneComponent.K2_SetWorldRotation` (`self.GeometryCollection`) (`KismetMathLibrary.MakeRotator` (`KismetMathLibrary.RandomFloatInRange` -180.0 180.0) (`KismetMathLibrary.RandomFloatInRange` -180.0 180.0) (`KismetMathLibrary.RandomFloatInRange` -180.0 180.0)) false false))
    (:`then_1`
      (`SceneComponent.SetWorldScale3D` (`self.GeometryCollection`) (`KismetMathLibrary.MakeVector` _returnvalue _returnvalue _returnvalue)))))

(fn `UserConstructionScript`)