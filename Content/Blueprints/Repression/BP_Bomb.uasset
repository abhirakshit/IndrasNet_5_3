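; BP_Bomb is a bomb that, on its Explode event, plays an explosion effect and sound, fractures and scatters physics objects, then destroys itself.
; It applies two Chaos field commands centered on its collision sphere: external cluster strain from a radial falloff to break clusters, then radial linear velocity to push pieces outward.
; A culling field limits the push to the sphere's radius.
; Nothing in this graph calls Explode.
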(event `Explode`
  (bind _returnvalue (`self.K2_GetActorLocation`))
  (bind _fieldsystemcomponent (`self.FieldSystemComponent`))
  (bind _spherecollision (`self.SphereCollision`))
  (bind _returnvalue_2 (`RadialFalloff.SetRadialFalloff` (`self.RadialFalloff`) (`self.Radial Falloff Magnitude`) 0.0 1.0 0.0 (`SphereComponent.GetScaledSphereRadius` _spherecollision) (`SceneComponent.K2_GetComponentLocation` _spherecollision) "Field_FallOff_None"))
  (`GameplayStatics.SpawnEmitterAtLocation` "/Game/StarterContent/Particles/P_Explosion.P_Explosion" _returnvalue (struct) (`KismetMathLibrary.Conv_DoubleToVector` (`self.Scale`)))
  (`GameplayStatics.PlaySoundAtLocation` "/Game/StarterContent/Audio/Explosion_Cue.Explosion_Cue" _returnvalue (struct) 0.2 0.2 0.0 null null null null)
  (`FieldSystemComponent.ApplyPhysicsField` _fieldsystemcomponent true "Field_ExternalClusterStrain" null _returnvalue_2)
  (`FieldSystemComponent.ApplyPhysicsField` _fieldsystemcomponent true "Field_LinearVelocity" null (`CullingField.SetCullingField` (`self.CullingField`) _returnvalue_2 (`RadialVector.SetRadialVector` (`self.RadialVector`) (`self.Radial Vector Magnitude`) (`SceneComponent.K2_GetComponentLocation` (`self.SphereCollision`))) "Field_Culling_Outside"))
  (`self.K2_DestroyActor`))

(fn `UserConstructionScript`)