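; Repression obstacle actor, a lava-material body with a loop sound that can act as a trap for tagged thought actors.
; On BeginPlay it picks a random mesh, rotation and scale, revealing it after a Niagara respawn effect.
; While trapping it overlaps, then blocks with a water material once a Reflected or Dissolving Thought exits; external events reset this or toggle visibility and audio.
; The hit-count dissolve chain is disconnected.
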(event `self.ReceiveBeginPlay`
  (bind _body (`self.Body`))
  (bind _body_2 (`self.Body`))
  (`|ExecutionSequence`
    (:`then_0`
      (bind _output_get (set `self.SMVal` (`KismetMathLibrary.RandomIntegerInRange` 0 2)))
      (switch `int` _output_get
        (:`0`
          (`StaticMeshComponent.SetStaticMesh` _body (`self.SM2`) :!label _label))
        (:`1`
          (`StaticMeshComponent.SetStaticMesh` _body (`self.SM1`)))
        (:`2`
          (goto _label)))
      (`SceneComponent.SetVisibility` _body_2 false false)
      (bind _returnvalue (`NiagaraFunctionLibrary.SpawnSystemAttached` "/Game/Assets/FX-Niagara/Dissolve-Respawn/NS_ReSpawnMesh_SM_9.NS_ReSpawnMesh_SM_9" _body_2 "None" (0.0 0.0 0.0) (struct) "KeepRelativeOffset"))
      (`NiagaraComponent.SetVariableFloat` _returnvalue "Duration" (`self.ParticleDuration`))
      (`NiagaraComponent.SetVariableFloat` _returnvalue "SpawnRate" (`self.SpawnRate`))
      (`NiagaraComponent.SetVariableStaticMesh` _returnvalue "None" (`StaticMeshComponent.StaticMesh` (`self.Body`)))
      (`NiagaraComponent.ReinitializeSystem` _returnvalue)
      (`KismetSystemLibrary.Delay` (+ (`self.ParticleDuration`) 0.5))
      (`SceneComponent.SetVisibility` (`self.Body`) true false))
    (:`then_1`
      (`self.SetTransform`))
    (:`then_2`
      (`self.SetCollisionProfiles`))))

(event `self.Body.OnComponentEndOverlap`
  (params (OverlappedComponent :type "PrimitiveComponent Object Reference") (OtherActor :type "Actor Object Reference") (OtherComp :type "PrimitiveComponent Object Reference") (OtherBodyIndex :type Integer))
  (bind _body (`self.Body`))
  (bind _output (`|GetArrayItem` (`Actor.Tags` OtherActor)))
  (switch `name` _output
    (:`reflectedIdea`
      (`KismetSystemLibrary.PrintText` (`KismetTextLibrary.Conv_NameToText` _output)))
    (:`reflectedThought`
      (if (`self.isTrapping`) :!label _label_2
        ;[1 1 1] Trapping
        (`PrimitiveComponent.SetCollisionProfileName` _body "BlockAll" true)
        (`PrimitiveComponent.SetMaterial` _body 0 "/Game/Assets/Materials/Water/M_Water_1.M_Water_1")))
    (:`dissolvingThought`
      (goto _label_2))))

(event `/Game/Blueprints/Interfaces/BP_RepressionInterface.ResetCollisionAndRepression`
  (`self.ResetCollisionAndMaterial`))

(event `/Game/Blueprints/Interfaces/BP_RepressionInterface.UpdateVisibility`
  (params (`isVisible?` :type Boolean))
  (`self.UpdateVisibliity` `isVisible?`))

(event `/Game/Blueprints/Interfaces/BP_RepressionInterface.UpdateTrapping`
  (params (`isTrapping?` :type Boolean))
  (set `self.isTrapping` `isTrapping?`)
  (`self.ResetCollisionAndMaterial`))

(event `self.Body.OnComponentHit`
  (params (HitComponent :type "PrimitiveComponent Object Reference") (OtherActor :type "Actor Object Reference") (OtherComp :type "PrimitiveComponent Object Reference") (NormalImpulse :type "Vector Structure") (Hit :type "HitResult Structure (by ref)"))
  (switch `name` (`|GetArrayItem` (`Actor.Tags` OtherActor))))

(fn `ResetCollisionAndMaterial`
  (`self.SetCollisionProfiles`)
  (`PrimitiveComponent.SetMaterial` (`self.Body`) 0 "/Game/Assets/Materials/Lava/MI_LavaRepressionDissolve.MI_LavaRepressionDissolve"))

(fn `SetCollisionProfiles`
  (bind _body (`self.Body`))
  (if (`self.isTrapping`)
    (`PrimitiveComponent.SetCollisionProfileName` _body "OverlapAll" true)
    (else
      (`PrimitiveComponent.SetCollisionProfileName` _body "BlockAll" true))))

(fn `SetTransform`
  (bind _returnvalue (`KismetMathLibrary.RandomFloatInRange` 1.5 2.5))
  (`|ExecutionSequence`
    (:`then_0`
      (`SceneComponent.K2_SetWorldRotation` (`self.Body`) (`KismetMathLibrary.MakeRotator` (`KismetMathLibrary.RandomFloatInRange` -180.0 180.0) (`KismetMathLibrary.RandomFloatInRange` -180.0 180.0) (`KismetMathLibrary.RandomFloatInRange` -180.0 180.0)) false false))
    (:`then_1`
      (`SceneComponent.SetWorldScale3D` (`self.Body`) (`KismetMathLibrary.MakeVector` _returnvalue _returnvalue _returnvalue)))))

(fn `ToggleAudio`
  (params (`play?` :type Boolean))
  (bind _lava_loop (`self.lava-loop`))
  (if `play?`
    (`AudioComponent.SetVolumeMultiplier` _lava_loop 1.0)
    (else
      (`AudioComponent.SetVolumeMultiplier` _lava_loop 0.0))))

(fn `UpdateVisibliity`
  (params (`isVisible?` :type Boolean))
  (bind _body (`self.Body`))
  (if `isVisible?`
    (`PrimitiveComponent.SetCollisionProfileName` _body "OverlapAll" true)
    (else
      (`PrimitiveComponent.SetCollisionProfileName` _body "NoCollision" true)))
  (`SceneComponent.SetVisibility` _body `isVisible?` false)
  (`self.ToggleAudio` `isVisible?`))

(fn `UserConstructionScript`)