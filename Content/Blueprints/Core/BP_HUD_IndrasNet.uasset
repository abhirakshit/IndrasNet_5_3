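; HUD for Indra's Net that creates the menu for the requested level (intro, playground or AI onboarding) and manages crosshairs and the mental model menu.
; For playground and onboarding, it spawns a BP_AI_Visualizer_Connector targeting the player controller's mental model and binds AI replies to the active widget.
; It forwards chat messages and prompt-profile changes to that connector, and retargets it when a mental model menu opens.
; It also relays skybox selections and timed messages to the main menu.
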(event `SetupOnboardingWidget`
  (`|ExecutionSequence`
    (:`then_0`
      (bind _returnvalue (`|CreateWidget` "/Game/Blueprints/Widgets/WBP_OnboardingAI.WBP_OnboardingAI_C"))
      (bind _output_get (set `self.WBOnboarding` _returnvalue))
      (`UserWidget.AddToViewport` _output_get 0))
    (:`then_1`
      (bind _aspc_indras_net (`self.GetPlayerController`))
      (bind _model (`/Game/Blueprints/Core/PC_IndrasNet.GetMentalModel` _aspc_indras_net))
      (bind _returnvalue_2 (`|SpawnActorFromClass` "/Game/Blueprints/ChatGPT/BP_AI_Visualizer_Connector.BP_AI_Visualizer_Connector_C" (`KismetMathLibrary.MakeTransform` (0.0 0.0 0.0)) "Undefined" "MultiplyWithRoot" null _model 0 null))
      (bind _output_get_2 (set `self.AIVizConnector` _returnvalue_2))
      (add `/Game/Blueprints/ChatGPT/BP_AI_Visualizer_Connector.RecievedMessageFromAI` _output_get_2 (delegate `ShowAIMsg`)))))

(event `ShowAIMsg`
  (params (Message :type String))
  (`/Game/Blueprints/Widgets/WBP_OnboardingAI.showAIResponse` (`self.WBOnboarding`) Message))

(event `self.ReceiveBeginPlay`
  (bind _asbp_default_player_indras_net (cast `/Game/Blueprints/Core/BP_DefaultPlayer_IndrasNet` (`GameplayStatics.GetPlayerPawn` 0)))
  (set `self.DefaultPlayer` _asbp_default_player_indras_net))

(event `SetupMainMenuWidget`
  (params (LevelName :type Name))
  ;[1 1 1] Add Menu - Call from PC
  (switch `name` LevelName
    (:`Level_Intro`
      (bind _returnvalue (`|CreateWidget` "/Game/Blueprints/Widgets/WBP_IntroMenu.WBP_IntroMenu_C"))
      (`UserWidget.AddToViewport` _returnvalue 0))
    (:`Level_Playground`
      (`self.SetupPlaygroundMenu`))
    (:`Level_OnboardingAI`
      (`self.SetupOnboardingWidget`))))

(event `UpdateSkyboxOption`
  (params (Selection :type Integer))
  (`/Game/Blueprints/Widgets/WBP_MainMenu.Update Skybox Setting` (`self.WBMainMenu`) Selection))

(event `SetupPlaygroundMenu`
  (`|ExecutionSequence`
    (:`then_0`
      (bind _returnvalue (`|CreateWidget` "/Game/Blueprints/Widgets/WBP_MainMenu.WBP_MainMenu_C"))
      (bind _output_get (set `self.WBMainMenu` _returnvalue))
      (`UserWidget.AddToViewport` _output_get 0))
    (:`then_1`
      (bind _aspc_indras_net (`self.GetPlayerController`))
      (bind _model (`/Game/Blueprints/Core/PC_IndrasNet.GetMentalModel` _aspc_indras_net))
      (bind _returnvalue_2 (`|SpawnActorFromClass` "/Game/Blueprints/ChatGPT/BP_AI_Visualizer_Connector.BP_AI_Visualizer_Connector_C" (`KismetMathLibrary.MakeTransform` (0.0 0.0 0.0)) "Undefined" "MultiplyWithRoot" null _model 1 null))
      (bind _output_get_2 (set `self.AIVizConnector` _returnvalue_2))
      (add `/Game/Blueprints/ChatGPT/BP_AI_Visualizer_Connector.RecievedMessageFromAI` _output_get_2 (delegate `CustomEvent`)))))

(event `CustomEvent`
  (params (Message :type String))
  (`/Game/Blueprints/Widgets/WBP_MainMenu.ShowAIResponse` (`self.WBMainMenu`) Message))

(event `SendMsgToAIConnector`
  (params (Message :type String))
  (`/Game/Blueprints/ChatGPT/BP_AI_Visualizer_Connector.SendMessageToAI` (`self.AIVizConnector`) Message))

(event `ShowMessage`
  (params (message :type Text) (hideTime :type "Float (double-precision)"))
  (bind _wbmainmenu (`self.WBMainMenu`))
  ;[1 1 1] Temp Message Display
  (`/Game/Blueprints/Widgets/WBP_MainMenu.DisplayHideMessage` _wbmainmenu message)
  (`KismetSystemLibrary.Delay` hideTime)
  (`/Game/Blueprints/Widgets/WBP_MainMenu.DisplayHideMessage` _wbmainmenu ""))

(event `UpdateAIPromptProfile`
  (params (Inp :type Integer))
  (`/Game/Blueprints/ChatGPT/BP_AI_Visualizer_Connector.SetGPTProfile` (`self.AIVizConnector`) Inp))

(fn `GetPlayerController`
  (returns (`AsPC Indras Net` :type "/Game/Blueprints/Core/PC_IndrasNet Object Reference"))
  (bind _aspc_indras_net (cast `/Game/Blueprints/Core/PC_IndrasNet` (`GameplayStatics.GetPlayerController` 0))
    (:`then`
      (return _aspc_indras_net))
    (:`CastFailed`
      (`KismetSystemLibrary.PrintText` "Error: HUD - PC Cast failed"))))

(fn `hideMentalModelMenu`
  (`/Game/Blueprints/Widgets/WBP_MainMenu.ToggleMentalModelMenuVisibility` (`self.WBMainMenu`) false null))

(fn `showHideCrosshairs`
  (params (show :type Boolean))
  (if show
    (if (not (`KismetSystemLibrary.IsValid` (`self.WBCrosshairREF`)))
      (bind _returnvalue (`|CreateWidget` "/Game/Blueprints/Widgets/WB_Crosshair.WB_Crosshair_C" (`GameplayStatics.GetPlayerController` 0)))
      (bind _output_get (set `self.WBCrosshairREF` _returnvalue)))
    (`UserWidget.AddToViewport` _output_get 0)
    (else
      (`Widget.RemoveFromParent` (`self.WBCrosshairREF`)))))

(fn `showMentalModelMenu`
  (params (MentalModel :type "/Game/Blueprints/MentalModels/BP_MentalModelDefault Object Reference"))
  (`/Game/Blueprints/MentalModels/BP_MentalModelDefault.getModelProperties` MentalModel)
  (`/Game/Blueprints/Widgets/WBP_MainMenu.ToggleMentalModelMenuVisibility` (`self.WBMainMenu`) true MentalModel)
  (set `/Game/Blueprints/ChatGPT/BP_AI_Visualizer_Connector.TargetMentalModel` MentalModel (`self.AIVizConnector`)))

(fn `UserConstructionScript`
  (`self.showHideCrosshairs` true))