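; Player controller for IndrasNet that manages mental model actors, scenarios, level menus and onboarding, routing UI and AI chat through the HUD.
; Mouse buttons toggle between look and cursor modes, with a camera-forward trace selecting tagged models.
; Models spawn ahead of the camera into a GUID-keyed map.
; Rama Save persists models, scenarios (skybox, player transform) and a master file, loaded or created in the construction script, tracking recent and default models.
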(event `self.ReceiveBeginPlay`
  (`|ExecutionSequence`
    (:`then_0`
      (bind _asbp_hud_indras_net (cast `/Game/Blueprints/Core/BP_HUD_IndrasNet` (`self.GetHUD`)))
      (set `self.HUD` _asbp_hud_indras_net))))

(event `SetupOnboardingAI`
  ;[1 1 1] Called By LVL Onboarding AI
  (bind _output_get (`self.GetHUDObject`))
  (bind _modelproperties (`self.GetDefaultProperties` (struct)))
  (`self.AddMentalModelToScene` _modelproperties)
  (`/Game/Blueprints/Core/BP_HUD_IndrasNet.SetupMainMenuWidget` _output_get "Level_OnboardingAI")
  (`/Game/Blueprints/Core/BP_HUD_IndrasNet.showHideCrosshairs` _output_get false)
  (`self.ToggleMouseControls` true))

(event `SendChatToAI`
  (params (UserInput :type String))
  (`/Game/Blueprints/Core/BP_HUD_IndrasNet.SendMsgToAIConnector` (`self.HUD`) UserInput))

(event `ShowPlaygroundMenuWidget`
  ;[1 1 1] Setup Playground Main Menu
  (bind _asbp_hud_indras_net (cast `/Game/Blueprints/Core/BP_HUD_IndrasNet` (`self.GetHUD`)))
  (bind _output_get (set `self.HUD` _asbp_hud_indras_net))
  (`/Game/Blueprints/Core/BP_HUD_IndrasNet.SetupMainMenuWidget` _output_get "Level_Playground"))

(event `self.ReceiveTick`
  (params (DeltaSeconds :type "Float (single-precision)"))
  (bind (_deltax _deltay) (`self.GetInputMouseDelta`))
  ;[1 1 1] Rotate Drag Object - TO BE DELETED
  (if (`self.rotateObj?`)
    (`/Engine/EditorBlueprintResources/StandardMacros.IsValid` (`self.TargetMentalModel`) :!label _label
      (:`Is Valid`
        (`self.K2_AddActorWorldRotation` (`self.TargetMentalModel`) (`KismetMathLibrary.MakeRotator` (* _deltax 10.0) (* _deltay 10.0)) false false)))))

(event `Key|MiddleMouseButton`
  (params (Key :type "Key Structure"))
  ;[1 1 1] Rotate Drag Object - TO BE DELETED
  (:`Pressed`
    (set `self.rotateObj?` true)
    (goto _label))
  (:`Released`
    (set `self.rotateObj?` false)))

(event `Key|T`
  (params (Key :type "Key Structure"))
  ;[1 1 1] Rotate Drag Object - TO BE DELETED
  (:`Pressed`
    (`/Engine/EditorBlueprintResources/StandardMacros.FlipFlop`
      (:`A`
        (set `self.transformObj?` true))
      (:`B`
        (set `self.transformObj?` true)))))

(event `ShowIntroMenuWidget`
  ;[1 1 1] Called By LVL Intro
  (bind _asbp_hud_indras_net (cast `/Game/Blueprints/Core/BP_HUD_IndrasNet` (`self.GetHUD`)))
  (bind _output_get (set `self.HUD` _asbp_hud_indras_net))
  (`/Game/Blueprints/Core/BP_HUD_IndrasNet.SetupMainMenuWidget` _output_get "Level_Intro"))

(event `Key|RightMouseButton`
  (params (Key :type "Key Structure"))
  (bind _hud (`self.HUD`))
  (:`Pressed`
    (`self.ToggleMouseControls` false)
    (`/Game/Blueprints/Core/BP_HUD_IndrasNet.showHideCrosshairs` _hud true)
    (`/Game/Blueprints/Core/BP_HUD_IndrasNet.ShowMessage` _hud "Game Mode Activated!" 2.0)))

(event `Key|LeftMouseButton`
  (params (Key :type "Key Structure"))
  (bind _targetmentalmodel (`self.TargetMentalModel`))
  (bind _hud (`self.HUD`))
  (bind _hud_2 (`self.HUD`))
  ;[1 1 1] Show/Hide Mental Model Menu
  (:`Released`
    (`self.ToggleMouseControls` true)
    (`/Game/Blueprints/Core/BP_HUD_IndrasNet.showHideCrosshairs` _hud_2 false)
    (`/Game/Blueprints/Core/BP_HUD_IndrasNet.ShowMessage` _hud_2 "PC: Mouse Control Activated!" 2.0)
    (`self.GetMentalModel`)
    (`/Engine/EditorBlueprintResources/StandardMacros.IsValid` _targetmentalmodel
      (:`Is Valid`
        (`/Game/Blueprints/Core/BP_HUD_IndrasNet.showMentalModelMenu` _hud _targetmentalmodel))
      (:`Is Not Valid`
        (`/Game/Blueprints/Core/BP_HUD_IndrasNet.hideMentalModelMenu` _hud)))))

(event `AddNewMentalModel`
  ;[1 1 1] Spawn New Model
  (bind _modelproperties (`self.GetDefaultProperties` (struct)))
  (`self.AddMentalModelToScene` _modelproperties))

(event `DeleteSelectedMentalModel`
  (bind _targetmentalmodel (`self.TargetMentalModel`))
  ;[1 1 1] Remove Model
  (`/Engine/EditorBlueprintResources/StandardMacros.IsValid` _targetmentalmodel
    (:`Is Valid`
      (`self.K2_DestroyActor` _targetmentalmodel))))

(fn `AddMentalModelToScene`
  (params (Props :type "/Game/Blueprints/Structs/ST_MentalModelProperties Structure"))
  (returns (Model :type "/Game/Blueprints/MentalModels/BP_MentalModelDefault Object Reference"))
  (bind _returnvalue (`GameplayStatics.GetPlayerCameraManager` 0))
  (bind _returnvalue_2 (`KismetMathLibrary.MakeTransform` (+ (`PlayerCameraManager.GetCameraLocation` _returnvalue) (* (`SceneComponent.GetForwardVector` (`PlayerCameraManager.TransformComponent` _returnvalue)) 500.0)) (struct) (`self.DefaultMentalModelScale`)))
  (bind _structout (setmembers `/Game/Blueprints/Structs/ST_MentalModelProperties` :`StructRef` Props :`Model_Transform` _returnvalue_2))
  (bind _returnvalue_3 (`|SpawnActorFromClass` "/Game/Blueprints/MentalModels/BP_MentalModelDefault.BP_MentalModelDefault_C" _returnvalue_2 "AdjustIfPossibleButAlwaysSpawn" "MultiplyWithRoot" null _structout null))
  (`BlueprintMapLibrary.Map_Add` (`self.MentalModelMap`) (`.Id_18_62F478F748169C70AD3810AA484AA993` (break `/Game/Blueprints/Structs/ST_MentalModelProperties` _structout)) _returnvalue_3)
  (return _returnvalue_3))

(fn `CleanJSONString`
  (params (Input :type String))
  (returns (Output :type String))
  (return (`KismetStringLibrary.Replace` Input "\\")))

(fn `DeleteMentalModelFromSystem`
  (params (FileName :type String))
  (locals (StaticModelProps :type "/Game/Blueprints/Core/BP_MentalModelsStaticData Object Reference"))
  (bind _hud (`self.HUD`))
  (bind _returnvalue (`RamaSaveLibrary.RamaSave_DeleteFile` (`KismetStringLibrary.Concat_StrStr` (`RamaSaveLibrary.RamaSavePaths_GameRootDirectory`) "Saved/MentalModels/" (`KismetStringLibrary.Replace` FileName " " "-") ".sav")))
  (if _returnvalue
    (`/Game/Blueprints/Core/BP_HUD_IndrasNet.ShowMessage` _hud "Model Deleted" 2.0)
    (else
      (`/Game/Blueprints/Core/BP_HUD_IndrasNet.ShowMessage` _hud "Model Delete Failed!" 2.0))))

(fn `DeleteScenario`
  (params (ScenarioName :type String))
  (bind _hud (`self.HUD`))
  (bind _returnvalue (`RamaSaveLibrary.RamaSave_DeleteFile` (`KismetStringLibrary.Concat_StrStr` (`RamaSaveLibrary.RamaSavePaths_GameRootDirectory`) "Saved/ScenarioFiles/" ScenarioName ".sav")))
  (if _returnvalue
    (`/Game/Blueprints/Core/BP_HUD_IndrasNet.ShowMessage` _hud "Scenario Deleted" 2.0)
    (else
      (`/Game/Blueprints/Core/BP_HUD_IndrasNet.ShowMessage` _hud "Delete Failed!" 2.0))))

(fn `GetAllMentalModelsInLevel`
  (returns (MentalModelMap :type "Map of Guid Structure to /Game/Blueprints/MentalModels/BP_MentalModelDefault Object Reference"))
  (return (`self.MentalModelMap`)))

(fn `GetDefaultProperties`
  (params (Transform :type "Transform Structure"))
  (returns (ModelProperties :type "/Game/Blueprints/Structs/ST_MentalModelProperties Structure"))
  (locals (Props :type "/Game/Blueprints/Structs/ST_MentalModelProperties Structure" :default (struct :`Title` "New Mental Model" :`Description` "New Description" :`Model_Transform` (struct :`Rotation` (struct :`W` 1.0) :`Translation` (0.0 0.0 0.0) :`Scale3D` (1.0 1.0 1.0)) :`Uncentered_Intensity` 1.0 :`RepressionProps` (struct :`count` 3 :`rep1_visible?` true :`rep2_visible?` true :`rep3_visible?` true) :`InnerLIghtProps` (struct :`intensity` 2.0 :`Visibility` true :`Color` (struct :`R` 1.0 :`G` 0.906319 :`B` 0.167915 :`A` 1.0)) :`ArousalProps` (struct :`intensity` 2.0 :`Visibility` true :`Color` (struct :`R` 0.685832 :`G` 1.0 :`B` 0.168186 :`A` 1.0)) :`OpennessProps` (struct :`intensity` 5.0 :`Visibility` true :`Color` (struct) :`ShieldColor` (struct)) :`CreatedAt` "0001.01.01-00.00.00" :`UpdatedAt` "0001.01.01-00.00.00")))
  (bind _returnvalue (`KismetMathLibrary.UtcNow`))
  (bind _structout (setmembers `/Game/Blueprints/Structs/ST_MentalModelProperties` :`StructRef` (`local.Props`) :`Id` (`KismetGuidLibrary.NewGuid`) :`Model_Transform` Transform :`CreatedAt` _returnvalue :`UpdatedAt` _returnvalue))
  (return _structout))

(fn `GetHUDObject`
  (returns (Output_Get :type "/Game/Blueprints/Core/BP_HUD_IndrasNet Object Reference"))
  (`/Engine/EditorBlueprintResources/StandardMacros.IsValid` (`self.HUD`)
    (:`Is Valid`
      _)
    (:`Is Not Valid`
      (bind _asbp_hud_indras_net (cast `/Game/Blueprints/Core/BP_HUD_IndrasNet` (`self.GetHUD`)))
      (set `self.HUD` _asbp_hud_indras_net)))
  (return (`self.HUD`)))

(fn `GetMasterGameFile`
  (returns (MasterGameProps :type "/Game/Blueprints/Core/BP_GameStaticData Object Reference"))
  (return (`self.MasterGameProps`)))

(fn `GetMentalModel`
  (returns (model :type "/Game/Blueprints/MentalModels/BP_MentalModelDefault Object Reference"))
  (locals (Return :type "/Game/Blueprints/Interfaces/BP_MentalModelInterface Interface"))
  (bind _returnvalue (`GameplayStatics.GetPlayerCameraManager` 0))
  (bind _returnvalue_2 (`PlayerCameraManager.GetCameraLocation` _returnvalue))
  (bind _outhit (`KismetSystemLibrary.LineTraceSingle` _returnvalue_2 (+ _returnvalue_2 (* (`SceneComponent.GetForwardVector` (`PlayerCameraManager.TransformComponent` _returnvalue)) (`self.Line Trace Length`))) "TraceTypeQuery1" false (`|MakeArray` self :!type "Actor Object Reference")))
  (if (`GameplayStatics.BreakHitResult` _outhit)
    (if (`self.ActorHasTag` (`.HitActor` (`GameplayStatics.BreakHitResult` _outhit)) "mentalModel")
      (bind _asbp_mental_model_default (cast `/Game/Blueprints/MentalModels/BP_MentalModelDefault` (`.HitActor` (`GameplayStatics.BreakHitResult` _outhit)))
        (:`then`
          (bind _output_get (set `self.TargetMentalModel` _asbp_mental_model_default))
          (return _output_get))
        (:`CastFailed`
          (`KismetSystemLibrary.PrintString` "PC: Cast Failed")))))
  ;[1 1 1] Set Null
  (bind _output_get_2 (set `self.TargetMentalModel` null))
  (return _output_get_2))

(fn `LoadDefaultUserMentalModel`
  (returns (Model :type "/Game/Blueprints/MentalModels/BP_MentalModelDefault Object Reference") (hasDefaultModel :type Boolean))
  (bind _mastergameprops (`self.MasterGameProps`))
  (bind _defaultusermodel (`/Game/Blueprints/Core/BP_GameStaticData.DefaultUserModel` _mastergameprops))
  (`/Engine/EditorBlueprintResources/StandardMacros.IsValid` _mastergameprops
    (:`Is Valid`
      (if (not (`KismetStringLibrary.IsEmpty` _defaultusermodel))
        (bind _model (`self.LoadMentalModelFromSystem` _defaultusermodel))
        (return _model true)
        (else
          ;[1 1 1] Remove Later
          (bind _modelproperties (`self.GetDefaultProperties` (struct)))
          (bind _model_2 (`self.AddMentalModelToScene` _modelproperties))
          (return _model_2 true))))
    (:`Is Not Valid`
      (`KismetSystemLibrary.PrintText` "PC:3 -  Load Mental Model Failed!!" true true (struct :`R` 1.0 :`G` 0.017294 :`B` 0.096967 :`A` 1.0) 10.0))))

(fn `LoadMasterGameFileFromSystem`
  (bind (_fileiosuccess _returnvalue) (`RamaSaveLibrary.RamaSave_LoadStaticDataFromFile` (`KismetStringLibrary.Concat_StrStr` (`RamaSaveLibrary.RamaSavePaths_GameRootDirectory`) "Saved/" "GameMaster" ".sav")))
  (if _fileiosuccess
    (bind _asbp_game_static_data (cast `/Game/Blueprints/Core/BP_GameStaticData` _returnvalue)
      (:`then`
        (set `self.MasterGameProps` _asbp_game_static_data)
        (`KismetSystemLibrary.PrintText` "PC: 1 - Successfuly loaded master game props" true true (struct :`G` 0.66 :`B` 1.0 :`A` 1.0) 10.0))
      (:`CastFailed`
        (`KismetSystemLibrary.PrintString` "PC Error: Could Not Load Master Game Props" true true (struct :`R` 1.0 :`G` 0.070812 :`B` 0.130541 :`A` 1.0) 10.0)))
    (else
      (bind _returnvalue_2 (`|GenericCreateObject` "/Game/Blueprints/Core/BP_GameStaticData.BP_GameStaticData_C"))
      (`self.SaveMasterGameFileToSystem` _returnvalue_2)
      (set `self.MasterGameProps` _returnvalue_2)
      (`KismetSystemLibrary.PrintText` "PC: Successfuly created master game props" true true (struct :`G` 0.66 :`B` 1.0 :`A` 1.0) 10.0))))

(fn `LoadMentalModelFromSystem`
  (params (FileName :type String))
  (returns (Model :type "/Game/Blueprints/MentalModels/BP_MentalModelDefault Object Reference"))
  (locals (StaticModelProps :type "/Game/Blueprints/Core/BP_MentalModelsStaticData Object Reference"))
  (bind (_fileiosuccess _returnvalue) (`RamaSaveLibrary.RamaSave_LoadStaticDataFromFile` (`KismetStringLibrary.Concat_StrStr` (`RamaSaveLibrary.RamaSavePaths_GameRootDirectory`) "Saved/MentalModels/" FileName ".sav")))
  (if _fileiosuccess
    (bind _asbp_mental_models_static_data (cast `/Game/Blueprints/Core/BP_MentalModelsStaticData` _returnvalue)
      (:`then`
        (bind _model (`self.AddMentalModelToScene` (`/Game/Blueprints/Core/BP_MentalModelsStaticData.MentalModelProperties` _asbp_mental_models_static_data)))
        (return _model))
      (:`CastFailed`
        (`KismetSystemLibrary.PrintString` "PC: Cast Failed Load mental model!")))
    (else
      (`/Game/Blueprints/Core/BP_HUD_IndrasNet.ShowMessage` (`self.HUD`) "Static Model File Load Failed!" 2.0))))

(fn `LoadMostRecentMentalModel`
  (returns (Model :type "/Game/Blueprints/MentalModels/BP_MentalModelDefault Object Reference"))
  (bind _mastergameprops (`self.MasterGameProps`))
  (bind _mostrecentupdatedmodel (`/Game/Blueprints/Core/BP_GameStaticData.MostRecentUpdatedModel` _mastergameprops))
  (`/Engine/EditorBlueprintResources/StandardMacros.IsValid` _mastergameprops
    (:`Is Valid`
      (if (not (`KismetStringLibrary.IsEmpty` _mostrecentupdatedmodel))
        (bind _model (`self.LoadMentalModelFromSystem` _mostrecentupdatedmodel))
        (return _model)
        (else
          (bind _modelproperties (`self.GetDefaultProperties` (struct)))
          (bind _model_2 (`self.AddMentalModelToScene` _modelproperties))
          (return _model_2))))
    (:`Is Not Valid`
      (`KismetSystemLibrary.PrintText` "PC:3 -  Load Mental Model Failed!!" true true (struct :`R` 1.0 :`G` 0.017294 :`B` 0.096967 :`A` 1.0) 10.0))))

(fn `LoadScenario`
  (params (ScenarioName :type String))
  (bind _staticscenariodata (`self.StaticScenarioData`))
  (bind _returnvalue (`KismetStringLibrary.Concat_StrStr` (`RamaSaveLibrary.RamaSavePaths_GameRootDirectory`) "Saved/ScenarioFiles/" (`self.LoadScenarioName`) ".sav"))
  (bind _skybackgroundselection (`/Game/Blueprints/Core/BP_ScenarioStaticData.SkyBackgroundSelection` (`self.StaticScenarioData`)))
  (set `self.LoadScenarioName` ScenarioName)
  (bind _fileiosuccess (`RamaSaveLibrary.RamaSave_LoadFromFile` _returnvalue))
  (if _fileiosuccess
    (bind (_fileiosuccess_2 _returnvalue_2) (`RamaSaveLibrary.RamaSave_LoadStaticDataFromFile` _returnvalue))
    (if _fileiosuccess_2
      (bind _asbp_scenario_static_data (cast `/Game/Blueprints/Core/BP_ScenarioStaticData` _returnvalue_2))
      (set `self.StaticScenarioData` _asbp_scenario_static_data)
      (`|ExecutionSequence`
        (:`then_0`
          (`self.UpdateSkyBoxMaterial` _skybackgroundselection)
          (`/Game/Blueprints/Core/BP_HUD_IndrasNet.UpdateSkyboxOption` (`self.HUD`) _skybackgroundselection))
        (:`then_1`
          (`self.K2_SetActorLocationAndRotation` (`GameplayStatics.GetPlayerController` 0) (`/Game/Blueprints/Core/BP_ScenarioStaticData.PlayerLocation` _staticscenariodata) (`/Game/Blueprints/Core/BP_ScenarioStaticData.PlayerRotation` _staticscenariodata) false false))
        (:`then_2`
          (`/Game/Blueprints/Core/BP_HUD_IndrasNet.ShowMessage` (`self.HUD`) "Scenario Loaded" 2.0)))
      (else
        (`/Game/Blueprints/Core/BP_HUD_IndrasNet.ShowMessage` (`self.HUD`) "Static File Load Failed!" 2.0)))
    (else
      (`/Game/Blueprints/Core/BP_HUD_IndrasNet.ShowMessage` (`self.HUD`) "File Load Failed!" 2.0))))

(fn `SaveMasterGameFileToSystem`
  (params (NewParam :type "/Game/Blueprints/Core/BP_GameStaticData Object Reference"))
  (bind _fileiosuccess (`RamaSaveLibrary.RamaSave_SaveOnlyStaticToFile` (`KismetStringLibrary.Concat_StrStr` (`RamaSaveLibrary.RamaSavePaths_GameRootDirectory`) "Saved/" "GameMaster" ".sav") NewParam))
  (if (not _fileiosuccess)
    (`KismetSystemLibrary.PrintString` "PC Error: Could not save Master Game File!")))

(fn `SaveMentalModelToSystem`
  (params (Guid :type "Guid Structure"))
  (locals (StaticModelProps :type "/Game/Blueprints/Core/BP_MentalModelsStaticData Object Reference") (ModelFileName :type String) (ModelFilePath :type String))
  (bind _hud (`self.HUD`))
  (bind _mastergameprops (`self.MasterGameProps`))
  (bind (_value _returnvalue) (`BlueprintMapLibrary.Map_Find` (`self.MentalModelMap`) Guid))
  (bind _modelpropertiesstruct (`/Game/Blueprints/MentalModels/BP_MentalModelDefault.ModelPropertiesStruct` _value))
  (bind _returnvalue_2 (`KismetStringLibrary.Replace` (`.Title_2_E0E7EE654786502B1B059180957414AE` (break `/Game/Blueprints/Structs/ST_MentalModelProperties` _modelpropertiesstruct)) " " "-"))
  (if _returnvalue
    (set `local.ModelFileName` _returnvalue_2)
    (set `local.ModelFilePath` (`KismetStringLibrary.Concat_StrStr` (`RamaSaveLibrary.RamaSavePaths_GameRootDirectory`) "Saved/MentalModels/" _returnvalue_2 ".sav"))
    (`|ExecutionSequence`
      (:`then_0`
        (bind _returnvalue_3 (`|GenericCreateObject` "/Game/Blueprints/Core/BP_MentalModelsStaticData.BP_MentalModelsStaticData_C" _modelpropertiesstruct))
        (set `local.StaticModelProps` _returnvalue_3))
      (:`then_1`
        (bind _fileiosuccess (`RamaSaveLibrary.RamaSave_SaveOnlyStaticToFile` (`local.ModelFilePath`) (`local.StaticModelProps`)))
        (if _fileiosuccess
          (`/Game/Blueprints/Core/BP_HUD_IndrasNet.ShowMessage` _hud "ModelSaved!" 2.0)
          (set `/Game/Blueprints/Core/BP_GameStaticData.MostRecentUpdatedModel` (`local.ModelFileName`) _mastergameprops)
          (`self.SaveMasterGameFileToSystem` _mastergameprops)
          (else
            (`/Game/Blueprints/Core/BP_HUD_IndrasNet.ShowMessage` _hud "Model Save Failed!" 2.0)))))
    (else
      (`KismetSystemLibrary.PrintString` "Model not found!"))))

(fn `SaveScenario`
  (params (ScenarioName :type String))
  (bind _hud (`self.HUD`))
  (`|ExecutionSequence`
    (:`then_0`
      (bind _returnvalue (`|GenericCreateObject` "/Game/Blueprints/Core/BP_ScenarioStaticData.BP_ScenarioStaticData_C" (`self.SkyBackgroundSelection`) "0.000000,0.000000,5.000000|0.000000,0.000000,0.000000|1.000000,1.000000,1.000000" (`self.K2_GetActorLocation` (`GameplayStatics.GetPlayerCharacter` 0)) (`self.GetControlRotation` (`GameplayStatics.GetPlayerController` 0))))
      (set `self.StaticScenarioData` _returnvalue))
    (:`then_1`
      (bind _fileiosuccess (`RamaSaveLibrary.RamaSave_SaveToFile` (`KismetStringLibrary.Concat_StrStr` (`RamaSaveLibrary.RamaSavePaths_GameRootDirectory`) "Saved/ScenarioFiles/" ScenarioName ".sav") "" false (`self.StaticScenarioData`)))
      (if _fileiosuccess
        (`/Game/Blueprints/Core/BP_HUD_IndrasNet.ShowMessage` _hud "ScenarioSaved!" 2.0)
        (else
          (`/Game/Blueprints/Core/BP_HUD_IndrasNet.ShowMessage` _hud "Save Failed!" 2.0))))))

(fn `SetDragRotateMode`
  (params (`drag?` :type Boolean))
  (bind _output_get (set `self.transformObj?` `drag?`))
  (set `self.rotateObj?` (not _output_get)))

(fn `SetDynamicSkyBox`
  (bind _returnvalue (`|SpawnActorFromClass` "/Game/Levels/SpaceSkyBox/BP_Sky_Sphere_Galaxy.BP_Sky_Sphere_Galaxy_C" (`KismetMathLibrary.MakeTransform` (0.0 0.0 0.0)) "Undefined" "MultiplyWithRoot" null "/Game/Levels/SpaceSkyBox/MI_Space_Dark.MI_Space_Dark" null))
  (set `self.SkyBox` _returnvalue))

(fn `SetLevel`
  (params (Level :type "LevelInstance Object Reference"))
  (set `self.CurrentLevel` Level))

(fn `StartOnboarding`
  (`|ExecutionSequence`
    (:`then_0`
      (bind _returnvalue (`|CreateWidget` "/Game/Blueprints/Widgets/WBP_OnboardingAI.WBP_OnboardingAI_C"))
      (bind _output_get (set `self.Widget_Onboarding` _returnvalue))
      (`UserWidget.AddToViewport` _output_get 0))
    (:`then_1`
      (bind _model (`self.LoadDefaultUserMentalModel`))
      (set `self.TargetMentalModel` _model))))

(fn `ToggleMouseControls`
  (params (showMouse :type Boolean :default true))
  (bind _returnvalue (`GameplayStatics.GetPlayerController` 0))
  (if showMouse
    (set `PlayerController.bShowMouseCursor` true _returnvalue)
    (`GameplayStatics.SetViewportMouseCaptureMode` "NoCapture")
    (`WidgetBlueprintLibrary.SetInputMode_GameAndUIEx` _returnvalue null "DoNotLock" false)
    (`self.SetIgnoreLookInput` _returnvalue true)
    (else
      (set `PlayerController.bShowMouseCursor` false _returnvalue)
      (`GameplayStatics.SetViewportMouseCaptureMode` "CapturePermanently_IncludingInitialMouseDown")
      (`WidgetBlueprintLibrary.SetInputMode_GameOnly` _returnvalue)
      (`self.ResetIgnoreLookInput` _returnvalue))))

(fn `UpdateAudioVolume`
  (params (newVol :type "Float (double-precision)"))
  (`AudioComponent.AdjustVolume` (`self.LevelSound`) 0.2 newVol "Linear"))

(fn `UpdateSkyBoxMaterial`
  (params (num :type Integer))
  (locals (NewMI :type "MaterialInstanceDynamic Object Reference"))
  (bind _newmi (`local.NewMI`))
  (bind _output_get (set `self.SkyBackgroundSelection` num))
  (`KismetSystemLibrary.PrintString` (`KismetStringLibrary.Conv_IntToString` _output_get))
  (bind _skybox (`self.SkyBox`)
    (:`then`
      (`|ExecutionSequence`
        (:`then_0`
          (`self.K2_DestroyActor` _skybox))
        (:`then_1`
          (bind _returnvalue (`KismetMaterialLibrary.CreateDynamicMaterialInstance` "/Game/Levels/SpaceSkyBox/MI_Space_Dark.MI_Space_Dark"))
          (set `local.NewMI` _returnvalue)
          (switch `int` (`self.SkyBackgroundSelection`)
            (:`Default`
              (`MaterialInstanceDynamic.SetTextureParameterValue` _newmi "SkyboxTexture" "/Game/Levels/SpaceSkyBox/8k_stars.8k_stars" :!label _label))
            (:`0`
              (`MaterialInstanceDynamic.SetTextureParameterValue` _newmi "SkyboxTexture" "/Game/Levels/SpaceSkyBox/TC_CrabNebula.TC_CrabNebula"))
            (:`1`
              (goto _label))
            (:`2`
              (`MaterialInstanceDynamic.SetTextureParameterValue` _newmi "SkyboxTexture" "/Game/Levels/SpaceSkyBox/TC_fantasy-style-galaxy-background.TC_fantasy-style-galaxy-background"))
            (:`3`
              (`MaterialInstanceDynamic.SetTextureParameterValue` _newmi "SkyboxTexture" "/Game/Levels/SpaceSkyBox/TC_ribbon-light-space.TC_ribbon-light-space")))
          (bind _returnvalue_2 (`|SpawnActorFromClass` "/Game/Levels/SpaceSkyBox/BP_Sky_Sphere_Galaxy.BP_Sky_Sphere_Galaxy_C" (`KismetMathLibrary.MakeTransform` (0.0 0.0 0.0) (struct :`Pitch` 90.0 :`Roll` 180.0)) "Undefined" "MultiplyWithRoot" null (`local.NewMI`) null))
          (set `self.SkyBox` _returnvalue_2)
          (`KismetSystemLibrary.PrintString` "Skybox Created"))))
    (:`else`
      (`KismetSystemLibrary.PrintString` "Not Valid"))))

(fn `UserConstructionScript`
  (`self.LoadMasterGameFileFromSystem`)
  (`KismetSystemLibrary.PrintText` "PC: COntruction Load mastyer game"))