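; BP_CreativeSpark is a spark actor that can be moved to a location and signals when a tagged actor touches it.
; AnimateTo plays a timeline that lerps the root from its current world location toward the target.
; The Collision overlap fires the OverlapCreativeSpark dispatcher for tagged actors, while the Sphere overlap only prints debug text.
; An unconnected random-wander loop remains in the graph and never runs.
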(event `self.ReceiveBeginPlay`)

(event `AnimateTo`
  (params (NewLoc :type "Vector Structure"))
  (bind (_direction _offsetalpha) (`Timeline|Timeline_Mvmt` :!via `PlayFromStart`)
    (:`Update`
      (`SceneComponent.K2_SetWorldLocation` (`self.DefaultSceneRoot`) (`KismetMathLibrary.VLerp` (`SceneComponent.K2_GetComponentLocation` (`self.DefaultSceneRoot`)) NewLoc _offsetalpha) false false))))

(event `self.Sphere.OnComponentBeginOverlap`
  (params (OverlappedComponent :type "PrimitiveComponent Object Reference") (OtherActor :type "Actor Object Reference") (OtherComp :type "PrimitiveComponent Object Reference") (OtherBodyIndex :type Integer) (bFromSweep :type Boolean) (SweepResult :type "HitResult Structure (by ref)"))
  (`KismetSystemLibrary.PrintText` "Overlap"))

(event `self.Collision.OnComponentBeginOverlap`
  (params (OverlappedComponent :type "PrimitiveComponent Object Reference") (OtherActor :type "Actor Object Reference") (OtherComp :type "PrimitiveComponent Object Reference") (OtherBodyIndex :type Integer) (bFromSweep :type Boolean) (SweepResult :type "HitResult Structure (by ref)"))
  (if (`self.ActorHasTag` OtherActor (`self.Tag`))
    (`self.OverlapCreativeSpark`)))

(fn `UserConstructionScript`)