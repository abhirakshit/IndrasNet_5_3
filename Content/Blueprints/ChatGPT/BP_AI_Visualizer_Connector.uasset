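; Connects ChatGPT, through an AIITK component, to a target mental model that visualizes the user's mental and emotional state.
; Messages join an Onboarding or Playground thread, both offering the same tool functions; streamed and final replies go to CallRecievedMessageFromAI.
; Tool calls set arousal, openness or withdrawal, or spawn reflected thoughts, then report success back to GPT for a follow-up.
; Repression updates only parse JSON; centeredness, honesty and deception are unhandled.
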(event `self.ReceiveBeginPlay`
  (`self.SetupPrompts`))

(event `self.AIITKComponentBP.OnGPTChunkReceived`
  (params (Completion :type "GPTChatCompletion Structure"))
  (`self.RecievedMessageFromAI` (`OpenAIFunctionLibrary.GetMessageContent` (`OpenAIFunctionLibrary.GetResponseMessage` Completion))))

(event `SendMessageToAI`
  (params (Message :type String))
  (bind _aiitkcomponentbp (`self.AIITKComponentBP`))
  (bind _gptrequestparamsthread (`self.GetGPTPrompt`))
  (`/AIIntegrationToolkit/Core/AIITKComponentBP.AddGPTUserMessage` _aiitkcomponentbp _gptrequestparamsthread Message)
  (`/AIIntegrationToolkit/Core/AIITKComponentBP.SendRequestToGPT` _aiitkcomponentbp _gptrequestparamsthread))

(event `self.AIITKComponentBP.OnGPTFailed`
  (params (ErrorMessage :type "GPTChatCompletion Structure"))
  (`self.RecievedMessageFromAI` (`OpenAIFunctionLibrary.GetMessageContent` (`OpenAIFunctionLibrary.GetResponseMessage` ErrorMessage))))

(event `self.AIITKComponentBP.OnGPTCompleted`
  (params (Completion :type "GPTChatCompletion Structure"))
  (bind _targetmentalmodel (`self.TargetMentalModel`))
  (bind _output_get (set `self.CurrentChatCompletion` Completion))
  (bind (_role _content _toolcalls) (break `AssistantMessage` (`.AssistantMessage` (break `GPTChatMessage` (`OpenAIFunctionLibrary.GetResponseMessage` _output_get)))))
  (set `self.CurrentToolCalls` _toolcalls)
  ;[1 1 1] Check if just message
  (if (`KismetStringLibrary.IsEmpty` _content)
    ;[1 1 1] Add Tool Message
    (if (> (`KismetArrayLibrary.Array_Length` _toolcalls) 0)
      (`self.AddAssistantToolMessage`)
      (for _array_element (`self.CurrentToolCalls`)
        (`|ExecutionSequence`
          (:`then_0`
            ;[1 1 1] Save FN Data
            (bind _output_get_2 (set `self.CurrentFunctionName` (`.FunctionName` (break `ToolCall` _array_element))))
            (bind _output (`self.CleanJSONString` (`.FunctionArguments` (break `ToolCall` _array_element))))
            (bind _output_get_3 (set `self.CurrentFunctionParams` _output))
            (`KismetSystemLibrary.PrintText` (`|FormatText` "{fName}: {params}" _output_get_2 _output_get_3) true true (struct :`G` 0.66 :`B` 1.0 :`A` 1.0) 20.0))
          (:`then_1`
            ;[1 1 1] Call Update on Mental Model
            (switch `string` (`self.CurrentFunctionName`)
              (:`updateVesselProperty`
                (bind _jsonobject (`EasyJsonAsyncLoadFromString.AsyncLoadFromString` (`self.CurrentFunctionParams`))
                  (:`Successed`
                    (`self.UpdateMentalModel` (`EasyJsonObject.ReadString` _jsonobject "propertyName" "") (`EasyJsonObject.ReadFloat` _jsonobject "propertyValue" 0.0) (`EasyJsonObject.ReadString` _jsonobject "propertyColor" "")))))
              (:`updateRepressionState`
                (`EasyJsonAsyncLoadFromString.AsyncLoadFromString` (`self.CurrentFunctionParams`)))
              (:`updateActions`
                (bind _jsonobject_2 (`EasyJsonAsyncLoadFromString.AsyncLoadFromString` (`self.CurrentFunctionParams`))
                  (:`Successed`
                    (bind _returnvalue (`EasyJsonObject.ReadString` _jsonobject_2 "actionName" ""))
                    (`KismetSystemLibrary.PrintText` (`|FormatText` "AS: {as}, AN: {an}" (`EasyJsonObject.ReadBool` _jsonobject_2 "actionState" false) _returnvalue) true true (struct :`G` 0.66 :`B` 1.0 :`A` 1.0) 20.0)
                    (switch `string` _returnvalue
                      (:`Reflection`
                        (`/Game/Blueprints/MentalModels/BP_MentalModelDefault.Spawn Reflected Thought` :`self` _targetmentalmodel :`ThoughtTag` "reflectedThought"))
                      (:`Intervention`
                        (`/Game/Blueprints/MentalModels/BP_MentalModelDefault.Spawn Reflected Thought` :`self` _targetmentalmodel :`ThoughtTag` "dissolvingThought"))
                      (:`Creative Idea`
                        (`/Game/Blueprints/MentalModels/BP_MentalModelDefault.Spawn Reflected Thought` :`self` _targetmentalmodel :`ThoughtTag` "reflectedIdea"))))))))
          (:`then_2`
            ;[1 1 1] Add Success msg in Queue
            (`self.AddToolResponseMessage` (`.ID` (break `ToolCall` _array_element)) (`BlueprintJsonLibrary.Conv_JsonObjectToPrettyString` (`BlueprintJsonLibrary.JsonMakeField` (`BlueprintJsonLibrary.JsonMake`) "vesselUpdated" (`BlueprintJsonLibrary.JsonMakeBool` true)))))))
      ;[1 1 1] Add Success msg back to ChatGPT
      (bind _gptrequestparamsthread (`self.GetGPTPrompt`))
      (`/AIIntegrationToolkit/Core/AIITKComponentBP.SendRequestToGPT` (`self.AIITKComponentBP`) _gptrequestparamsthread))
    (else
      ;[1 1 1] Add Assistant Message
      (`self.AddAssistantTextMessage` (`OpenAIFunctionLibrary.GetMessageContent` (`OpenAIFunctionLibrary.GetResponseMessage` _output_get))))))

(fn `AddAssistantTextMessage`
  (params (Content :type String))
  (bind _gptrequestparamsthread (`self.GetGPTPrompt`))
  (`KismetArrayLibrary.Array_Add` (`.Messages` (break `GPTChatPromptParams` _gptrequestparamsthread)) (make `GPTChatMessage` :`Role` "assistant" :`AssistantMessage` (make `AssistantMessage` Content)))
  (`self.RecievedMessageFromAI` Content))

(fn `AddAssistantToolMessage`
  (bind _gptrequestparamsthread (`self.GetGPTPrompt`))
  (`KismetArrayLibrary.Array_Add` (`.Messages` (break `GPTChatPromptParams` _gptrequestparamsthread)) (make `GPTChatMessage` :`Role` "assistant" :`AssistantMessage` (make `AssistantMessage` "" (`self.CurrentToolCalls`)))))

(fn `AddToolResponseMessage`
  (params (`Tool Call ID` :type String) (Content :type String))
  (bind _gptrequestparamsthread (`self.GetGPTPrompt`))
  (`KismetArrayLibrary.Array_Add` (`.Messages` (break `GPTChatPromptParams` _gptrequestparamsthread)) (make `GPTChatMessage` :`Role` "tool" :`Name` (`self.CurrentFunctionName`) :`ToolMessage` (make `ToolMessage` Content `Tool Call ID`))))

(fn `CleanJSONString`
  (params (Input :type String))
  (returns (Output :type String))
  (return (`KismetStringLibrary.Replace` Input "\\")))

(fn `GetGPTFunctions`
  (returns (GPTChatToolParams :type "GPTChatToolParams Structure"))
  (return (make `GPTChatToolParams` (struct :`FunctionCallMode` "Null" :`SpecificFunctionName` "My_Function") (`|MakeArray` (make `GPTChatFunction` :`Name` "updateVesselProperty" :`Description` "Update the vessel property based on the user's mental and emotional state data input" :`RawJsonParameters` (`|MakeArray` (`|MakeGPTParameter` false "String" "propertyName" "Choose a property from 'arousal', 'withdrawal', 'openness', 'centeredness', 'honesty', 'deception'" true) (`|MakeGPTParameter` false "Number" "propertyValue" "A number between 1 and 5. The number can be a float value. 1 means very low and 5 means very high" true) (`|MakeGPTParameter` false "String" "propertyColor" "Provide a color HEX code matching their current emotional valence" true) "")) (make `GPTChatFunction` :`Name` "updateRepressionState" :`Description` "Update the repression vessel property based on the user input" :`RawJsonParameters` (`|MakeArray` (`|MakeGPTParameter` false "Boolean" "repressionVisibility" "Show or Hide repression" true) (`|MakeGPTParameter` false "String" "repressionState" "Pick one from 'Reflect', 'Ruminate', 'Dissolve' based on user inputs" true) (`|MakeGPTParameter` false "Number" "repressionNum" "Pick a number between 1 and 3. A user can show at max 3 repressions at one time" true))) (make `GPTChatFunction` :`Name` "updateActions" :`Description` "Start or stop actions like reflection, creative idea, intervention" :`RawJsonParameters` (`|MakeArray` (`|MakeGPTParameter` false "Boolean" "actionState" "Start or Stop Action" true) (`|MakeGPTParameter` false "String" "actionName" "Pick one from 'Reflection', 'Intervention', 'Creative Idea' based on user inputs" true)))))))

(fn `GetGPTPrompt`
  (returns (GPTRequestParamsThread :type "GPTChatPromptParams Structure"))
  (switch `int` (`self.ChatGPTPromptSelection`)
    (:`0`
      (return (`self.GPTRequestParamsThreadOnboarding`)))
    (:`1`
      (return (`self.GPTRequestParamsThreadPlayground`)))))

(fn `SetupPrompts`
  (`|ExecutionSequence`
    (:`then_0`
      (bind _gptchattoolparams (`self.GetGPTFunctions`))
      (bind _structout (setmembers `GPTChatPromptParams` :`StructRef` (`self.GPTRequestParamsThreadOnboarding`) :`ToolParams` _gptchattoolparams))
      (set `self.GPTRequestParamsThreadOnboarding` _structout))
    (:`then_1`
      (bind _gptchattoolparams_2 (`self.GetGPTFunctions`))
      (bind _structout_2 (setmembers `GPTChatPromptParams` :`StructRef` (`self.GPTRequestParamsThreadPlayground`) :`ToolParams` _gptchattoolparams_2))
      (set `self.GPTRequestParamsThreadPlayground` _structout_2))))

(fn `SetupTargetMentalModel`
  (params (TargetMentalModel :type "/Game/Blueprints/MentalModels/BP_MentalModelDefault Object Reference"))
  (set `self.TargetMentalModel` TargetMentalModel))

(fn `UpdateMentalModel`
  (params (PropertyName :type String) (Value :type "Float (double-precision)") (Color :type String))
  (locals (ErrorColor :type "LinearColor Structure" :default (struct :`R` 1.0 :`G` 0.107261 :`B` 0.939577 :`A` 1.0)))
  (bind _targetmentalmodel (`self.TargetMentalModel`))
  (bind _returnvalue (`Helpers.HexToLinearColor` (`KismetTextLibrary.Conv_StringToText` Color) (`local.ErrorColor`)))
  (switch `string` PropertyName
    (:`arousal`
      (`/Game/Blueprints/MentalModels/BP_MentalModelDefault.UpdateArousalProps` _targetmentalmodel Value true _returnvalue))
    (:`openness`
      (`/Game/Blueprints/MentalModels/BP_MentalModelDefault.UpdateOpennessProps` _targetmentalmodel Value false _returnvalue))
    (:`withdrawal`
      (`/Game/Blueprints/MentalModels/BP_MentalModelDefault.UpdateWithdrawalProps` _targetmentalmodel Value (`KismetMathLibrary.RandomBool`) _returnvalue))))

(fn `UserConstructionScript`)